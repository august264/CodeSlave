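; BP_SpectatorCamController is a controller that previews tile-based object placement when the game mode's ToggleObjectPlacementDebug flag is on.
; On BeginPlay it spawns a BP_NEWTABLE at the origin as the placeable object.
; Each tick it traces under the cursor, snaps hits on MyMapManagerActor to tile positions via world-to-index-to-world conversion, and moves the table slightly above that tile.
; Debug strings print hit results and tile indices.
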(event EventBeginPlay
  ;[1 1 1] Read gameMode value
  (bind _asbp_game_mode_basic (Utilities|Casting|CastToBP_GameModeBasic (Game|GetGameMode)))
  (if (Variables|/Game/GameMode/BP_GameModeBasic.BP_GameModeBasic_C|GetToggle%20Object%20Placement%20Debug _asbp_game_mode_basic)
    ;[1 1 1] Spawn a Table actor
    (bind _returnvalue (Game|SpawnActorfromClass "/Game/testFiles/MapsAndObjects/BP_NEWTABLE.BP_NEWTABLE_C" (Math|Conversions|ToTransform(Vector) (Math|Vector|MakeVector 0.0 0.0 0.0)) "AlwaysSpawn" 0 0))
    (bind _output_get (Variables|Default|SetPlaceAbleObj _returnvalue))))

(event EventTick
  (params (DeltaSeconds :type Float%20%28single-precision%29))
  (bind _objects (Variables|Default|GetObjects))
  (bind _hitresult (Class|PlayerController|GetHitResultUnderCursorforObjects _objects true))
  (bind (_bblockinghit _binitialoverlap _time _distance _location _impactpoint _normal _impactnormal _physmat _hitactor) (Collision|BreakHitResult _hitresult))
  ;[1 1 1] Read gameMode value
  (bind _asbp_game_mode_basic (Utilities|Casting|CastToBP_GameModeBasic (Game|GetGameMode)))
  (if (Variables|/Game/GameMode/BP_GameModeBasic.BP_GameModeBasic_C|GetToggle%20Object%20Placement%20Debug _asbp_game_mode_basic)
    ;[1 1 1] Get Object under the mouse cursor
    ;;[1 1 1] Try to cast the actor to map actor
    (bind _asmy_map_manager_actor (Utilities|Casting|CastToMyMapManagerActor _hitactor)
      (:then
        ;[1 1 1] Debug output
        (Development|PrintString "Success")
        (Development|PrintString (Utilities|String|ToString(Vector) _location))
        ;[1 1 1] Transfer unbounded 3d cursor location to bounded tile location
        (bind _returnvalue (Class|MapManagerActor|GetTileIndexfromWorldPosition _asmy_map_manager_actor _location))
        (Development|PrintString (Utilities|String|ToString(Vector2d) _returnvalue))
        (bind _returnvalue_2 (Class|MapManagerActor|GetTileWorldPositon _asmy_map_manager_actor (Math|Float|Truncate (.X (Math|Vector2D|BreakVector2D _returnvalue))) (Math|Float|Truncate (.Y (Math|Vector2D|BreakVector2D _returnvalue)))))
        ;[1 1 1] Set the actor to that location
        (Transformation|SetActorLocation (stale EventBeginPlay _output_get) (+ _returnvalue_2 "0, 0,20.000000") false false))
      (:CastFailed
        (Development|PrintString (Utilities|GetDisplayName _hitactor))))))

(fn ConstructionScript)