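; BP_Employee is an employee pawn that generates random staff attributes and wanders the level.
; On BeginPlay, CreateStaff randomizes experience and age and passes a random 0-or-1 value to SetEmployeeName, then the results are printed as debug strings.
; Roam uses AI MoveTo toward random navigable points near its current location, re-calling itself on success, so a failed move ends the wandering.
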(event Custom|Roam
  (AI|AIMoveTo self (.RandomLocation (Class|NavigationSystem|GetRandomPointinNavigableRadius (Transformation|GetActorLocation) 2e+02)) 0 5.0 true
    (:OnSuccess
      (CallFunction|Roam))))

(event EventBeginPlay
  (CallFunction|CreateStaff)
  (bind _returnvalue (Class|Employee|GetExperience))
  (Development|PrintString (Utilities|String|ToString(Float) _returnvalue))
  (bind _returnvalue_2 (Class|Employee|GetAge))
  (Development|PrintString (Utilities|String|ToString(Integer) _returnvalue_2))
  (Development|PrintString (Variables|Default|GetemployeeName))
  (CallFunction|Roam))

(fn ConstructionScript)

(fn CreateStaff
  (Class|Employee|SetExperience (Math|Conversions|ToFloat(Integer) (Math|Random|RandomIntegerinRange 1 15)))
  (Class|Employee|SetAge (Math|Random|RandomIntegerinRange 18 65))
  (Class|Employee|SetEmployeeName (Math|Random|RandomIntegerinRange 0 1)))