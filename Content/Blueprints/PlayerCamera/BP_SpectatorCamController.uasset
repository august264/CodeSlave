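; Spectator camera player controller that previews buildable objects on a tile map under the mouse cursor.
; SetObject_Event spawns the given class as ObjToBuild, and every Tick calls Snap while that actor is valid.
; Snap traces under the cursor, converts the hit on MyMapManagerActor to a tile index, and moves the object to that tile's position with a height offset.
; FloorPlacement_Event only checks for a Floor type without acting on it.
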(event EventTick
  (params (DeltaSeconds :type Float%20%28single-precision%29))
  (if (Utilities|IsValid (Variables|Default|GetobjToBuild))
    (CallFunction|Snap)))

(event Custom|FloorPlacement_Event
  (bind _objtobuild (Variables|Default|GetobjToBuild))
  (Utilities|IsValid _objtobuild
    (:Is%20Valid
      (if (Utilities|Enum|Equal(Enum) (Variables|/Script/CodeSlave.TileObject|GetObjectTypes _objtobuild) "Floor")
        _))))

(event Custom|SetObject_Event
  (params (NewParam :type Tile%20Object%20Class%20Reference))
  (bind _returnvalue (Game|SpawnActorfromClass NewParam (Math|Transform|MakeTransform "0, 0, 0") "AdjustIfPossibleButAlwaysSpawn" 0 0))
  (Variables|Default|SetobjToBuild _returnvalue))

(fn ConstructionScript)

(fn Snap
  (bind _objects (Variables|Default|GetObjects))
  (bind _hitresult (Class|PlayerController|GetHitResultUnderCursorforObjects _objects true))
  (bind (_bblockinghit _binitialoverlap _time _distance _location _impactpoint _normal _impactnormal _physmat _hitactor) (Collision|BreakHitResult _hitresult))
  ;[1 1 1] Get Object under the mouse cursor
  ;;[1 1 1] Try to cast the actor to map actor
  (bind _asmy_map_manager_actor (Utilities|Casting|CastToMyMapManagerActor _hitactor))
  ;[1 1 1] Transfer unbounded 3d cursor location to bounded tile location
  (bind _returnvalue (Class|MapManagerActor|GetTileIndexfromWorldPosition _asmy_map_manager_actor _location))
  (bind _returnvalue_2 (Class|MapManagerActor|GetTileWorldPositon _asmy_map_manager_actor (Math|Float|Truncate (.X (Math|Vector2D|BreakVector2D _returnvalue))) (Math|Float|Truncate (.Y (Math|Vector2D|BreakVector2D _returnvalue)))))
  ;[1 1 1] Set the actor to that location
  (Transformation|SetActorLocation (Variables|Default|GetobjToBuild) (+ _returnvalue_2 "0, 0,60.000000") false false))