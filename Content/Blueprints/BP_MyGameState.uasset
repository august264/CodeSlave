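; Game state Blueprint that runs an in-game clock and calendar, from seconds up to years.
; Tick passes through a TimeRate Delay to increment Second, cascading overflow into Minute, Hour, Day, Month and Year.
; Day rollover branches on month length, using the IfLeapYear helper to apply the Gregorian leap-year rule to February.
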(event EventTick
  (params (DeltaSeconds :type Float%20%28single-precision%29))
  (bind _year (Variables|Default|GetYear))
  (Utilities|FlowControl|Delay (Variables|Default|GetTimeRate))
  (bind _result (Math|Integer|IncrementInt (Variables|Default|GetSecond))
    (:%20%20
      (if (>= _result 60)
        (bind _result_2 (Math|Integer|IncrementInt (Variables|Default|GetMinute))
          (:%20%20
            (Variables|Default|SetSecond 0)
            (if (>= _result_2 60)
              (bind _result_3 (Math|Integer|IncrementInt (Variables|Default|GetHour))
                (:%20%20
                  (Variables|Default|SetMinute 0)
                  (if (>= _result_3 24)
                    (bind _result_4 (Math|Integer|IncrementInt (Variables|Default|GetDay))
                      (:%20%20
                        (Variables|Default|SetHour 0)
                        (if (and (> _result_4 31) (Math|Boolean|ORBoolean (== (Variables|Default|GetMonth) 1) (== (Variables|Default|GetMonth) 3) (== (Variables|Default|GetMonth) 5) (== (Variables|Default|GetMonth) 7) (== (Variables|Default|GetMonth) 8) (== (Variables|Default|GetMonth) 10) (== (Variables|Default|GetMonth) 12)))
                          (bind _result_5 (Math|Integer|IncrementInt (Variables|Default|GetMonth))
                            (:%20%20
                              (Variables|Default|SetDay 1)
                              (if (> _result_5 12)
                                (Variables|Default|SetMonth 1)
                                (Math|Integer|IncrementInt _year))))
                          (elif (and (>= _result_4 30) (Math|Boolean|ORBoolean (== (Variables|Default|GetMonth) 4) (== (Variables|Default|GetMonth) 6) (== (Variables|Default|GetMonth) 9) (== (Variables|Default|GetMonth) 11)))
                            (bind _result_6 (Math|Integer|IncrementInt (Variables|Default|GetMonth))
                              (:%20%20
                                (Variables|Default|SetDay 1)
                                (if (> _result_6 12)
                                  (Variables|Default|SetMonth 1)
                                  (Math|Integer|IncrementInt _year))))
                            (else
                              ;[1 1 1] not a leap year
                              (bind _bisleap (CallFunction|IfLeapYear (Variables|Default|GetYear)))
                              (if (Math|Boolean|ANDBoolean (> _result_4 28) (Math|Boolean|Equal(Boolean) _bisleap false) (== (Variables|Default|GetMonth) 2))
                                (bind _result_7 (Math|Integer|IncrementInt (Variables|Default|GetMonth) :!label _label)
                                  (:%20%20
                                    (Variables|Default|SetDay 1)
                                    (if (> _result_7 12)
                                      (Variables|Default|SetMonth 1)
                                      (Math|Integer|IncrementInt (Variables|Default|GetYear)))))
                                (else
                                  (bind _bisleap_2 (CallFunction|IfLeapYear (Variables|Default|GetYear)))
                                  (if (Math|Boolean|ANDBoolean (> _result_4 29) (Math|Boolean|Equal(Boolean) _bisleap_2 true) (== (Variables|Default|GetMonth) 2))
                                    (goto _label)))))))))))))))))))

(fn ConstructionScript)

(fn IfLeapYear
  (params (Year :type Integer))
  (if (or (and (== (Math|Integer|%(Integer) Year 4) 0) (!= (Math|Integer|%(Integer) Year 100) 0)) (and (== (Math|Integer|%(Integer) Year 100) 0) (== (Math|Integer|%(Integer) Year 400) 0)))
    (return true)
    (else
      (return false))))