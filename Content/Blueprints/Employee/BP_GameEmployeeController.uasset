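; AI controller for game employee pawns that sends each one to a free tile to perform an action.
; After a one-second BeginPlay delay to let the pawn land, roaming claims the first unoccupied TileObject by setting its Occupied flag.
; It moves the pawn to that tile's TargetPoint, then on success triggers the Static_Face_Up action after a short pause.
; This graph neither releases tiles nor repeats roaming.
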(event EventBeginPlay
  ;[1 1 1] Because the character may spawn in the air, delay 1 sec to let it touches the ground before start the roaming event, otherwise, roaming will fail
  (Utilities|FlowControl|Delay 1.0)
  (CallFunction|RoamingEvent))

(event EventTick
  (params (DeltaSeconds :type Float%20%28single-precision%29)))

(event Custom|Roaming_Event
  (bind _astestaicharacter (Utilities|Casting|CastToTESTAICharacter (Pawn|GetControlledPawn)))
  (bind _outactors (Actor|GetAllActorsOfClass "/Script/CodeSlave.TileObject"))
  (bind _array_element (Utilities|Array|ForEachLoopwithBreak _outactors :!label _label)
    (:LoopBody
      (if (not (Variables|/Script/CodeSlave.TileObject|GetbOccupied _array_element))
        (Variables|/Script/CodeSlave.TileObject|SetbOccupied _array_element true)
        (AI|AIMoveTo _astestaicharacter (Transformation|GetWorldLocation (Variables|/Script/CodeSlave.TileObject|GettargetPoint _array_element)) 0 5.0 false
          (:then
            (goto _label Break))
          (:OnSuccess
            (bind _asbp_game_employee_actor (Utilities|Casting|CastToBP_GameEmployeeActor (Pawn|GetControlledPawn)))
            (Utilities|FlowControl|Delay 0.5)
            (Class|TESTAICharacter|ExcuteAction _asbp_game_employee_actor "Static_Face_Up")))))))

(fn ConstructionScript)