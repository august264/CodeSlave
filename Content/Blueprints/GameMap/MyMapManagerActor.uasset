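; Map manager actor that builds the game map's tile-based background and grid overlay.
; Its construction script calls TileMapSetUp, then loops over the map's X and Y size to fill the GridLine tile map with grid tiles.
; Inside the same loop it tints the grid cyan and assigns TerrainGround as the BackGround tile map.
; The event graph has no active logic.
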(event EventBeginPlay)

(event Collision|EventActorBeginOverlap
  (params (OtherActor :type Actor%20Object%20Reference)))

(event EventTick
  (params (DeltaSeconds :type Float%20%28single-precision%29)))

(fn ConstructionScript
  (Class|MapManagerActor|TileMapSetUp)
  (for _index (range 0 (Variables|Default|GetmapSizeX))
    (for _index_2 (range 0 (Variables|Default|GetmapSizeY))
      (Class|PaperTileMapComponent|SetTile (Variables|Default|GetgridLine) _index _index_2 0 (Variables|Default|GetGridLineInfo))
      (Class|PaperTileMapComponent|SetTileMapColor (Variables|Default|GetgridLine) "(R=0.119653,G=0.985078,B=1.000000,A=1.000000)")
      (Class|PaperTileMapComponent|SetTileMap (Variables|Default|GetBackGround) "/Game/Blueprints/GameMap/TerrainGround.TerrainGround"))))